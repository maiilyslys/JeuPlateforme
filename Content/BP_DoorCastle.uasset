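; BP_DoorCastle is an interactable double wooden castle door that requires the player character to hold a key.
; On Interact with the key, a FlipFlop alternates between two timelines, each swinging one leaf open 90 degrees: right first, then left on the next interaction.
; The right timeline also fires a desert ambience sound on every update.
; Without the key, it calls PlaySound2D with no sound assigned.
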(event `/Game/Input/Touch/BPI_Interact.Interact`
  (bind _asbp_third_person_character (cast `/Game/ThirdPerson/Blueprints/BP_ThirdPersonCharacter` (`GameplayStatics.GetPlayerCharacter` 0)))
  (if (`/Game/ThirdPerson/Blueprints/BP_ThirdPersonCharacter.Haskey` _asbp_third_person_character)
    (`/Engine/EditorBlueprintResources/StandardMacros.FlipFlop`
      (:`A`
        (bind (_direction _ouverture) (`Timeline|Timeline` :!via `PlayFromStart`)
          (:`Update`
            (`SceneComponent.K2_SetRelativeRotation` (`self.SM_door_wood_right`) (`KismetMathLibrary.MakeRotator` 0.0 0.0 (`KismetMathLibrary.Lerp` 0.0 -90.0 _ouverture)) false false)
            (`GameplayStatics.PlaySound2D` "/Game/SmallSoundKit/SSKCue/AmbienceCue/Amb_Desert_01_Cue.Amb_Desert_01_Cue" 1.0 1.0 0.0 null null))))
      (:`B`
        (bind (_direction_2 _ouverture_2) (`Timeline|Timeline_0` :!via `PlayFromStart`)
          (:`Update`
            (`SceneComponent.K2_SetRelativeRotation` (`self.SM_door_wood_left`) (`KismetMathLibrary.MakeRotator` 0.0 0.0 (`KismetMathLibrary.Lerp` 0.0 90.0 _ouverture_2)) false false)))))
    (else
      (`GameplayStatics.PlaySound2D` null 1.0 1.0 0.0 null null))))

(fn `UserConstructionScript`)